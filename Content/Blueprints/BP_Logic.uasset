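; Blackjack game controller that runs betting, hit, stand and double, payouts, and round or game end on bankruptcy or low deck.
; It spawns BP_Card actors from a shuffled multi-deck ID array, fanning them alternately left and right.
; Card values decode arithmetically from IDs, with aces dropping from 11 to 1 on bust.
; The dealer AI redraws through an event loop until 17, then hands are compared and results go to the HUD.
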(event `InitialSetup`
  (params (NoOfDecks :type Integer))
  ;[1 1 1] New game
  (set `self.NoOfDecks` NoOfDecks)
  (set `self.Show player hand value` false)
  (set `self.Show AI hand value` false))

(event `SendSuffledDeck`
  (params (NewParam :type "Array of Integer"))
  ;[1 1 1] New game
  (set `self.Card Deck Shuffled` NewParam))

(event `Create Card`
  (bind _no_of_cards_in_hand (`self.No of cards in hand`))
  (bind _card_x_location (`self.Card x location`))
  (bind _playershandvalue (`self.PlayersHandValue`))
  (bind _returnvalue (`KismetMathLibrary.FClamp` _card_x_location -1.0))
  ;[1 1 1] Player Cards placing
  (switch `int` _no_of_cards_in_hand
    (:`0`
      (set `self.Card x location` -50.0))
    (:`1`
      (set `self.Card x location` (* (+ (`KismetMathLibrary.Abs` _card_x_location) (* 1 110.0)) (* _returnvalue -1.0)) :!label _label))
    (:`2`
      (goto _label))
    (:`3`
      (goto _label))
    (:`4`
      (goto _label))
    (:`5`
      (goto _label))
    (:`6`
      (goto _label))
    (:`7`
      (goto _label))
    (:`8`
      (goto _label)))
  (set `self.No of cards in hand` (+ _no_of_cards_in_hand 1))
  (set `self.AutoRotate` true)
  (set `self.CardID` (`KismetArrayLibrary.Array_Get` (`self.Card Deck Shuffled`) (`self.Index`)))
  (bind _returnvalue_2 (`|SpawnActorFromClass` "/Game/Blueprints/BP_Card.BP_Card_C" (`KismetMathLibrary.Conv_VectorToTransform` (`KismetMathLibrary.MakeVector` _card_x_location 1100.0 (+ (* _returnvalue -1.0) (* _no_of_cards_in_hand 1.0)))) false (`self.CardID`) (`self.AutoRotate`) self))
  ;[1 1 1] Calculate players hand
  (set `self.Index` (+ (`self.Index`) 1))
  (`KismetArrayLibrary.Array_Add` (`self.CardsInHand`) _returnvalue_2)
  (set `self.CardIndexInHand` (+ (`self.CardIndexInHand`) 1))
  (bind (_cardvalue _ace) (`self.CalculateCardvalue` (`self.CardID`)))
  (if _ace
    (set `self.Player hand aces` (+ (`self.Player hand aces`) 1)))
  (set `self.PlayersHandValue` (+ _cardvalue _playershandvalue))
  (`/Engine/EditorBlueprintResources/StandardMacros.CompareInt` _playershandvalue 21 :!label _label_2
    (:`>`
      ;;[1 1 1] Check if player have aces
      (`/Engine/EditorBlueprintResources/StandardMacros.CompareInt` (`self.Player hand aces`)
        (:`>`
          (set `self.PlayersHandValue` (- (`self.PlayersHandValue`) 10))
          (set `self.Player hand aces` (- (`self.Player hand aces`) 1))
          (goto _label_2))
        (:`==`
          (`self.PlayerOver21points`))))
    (:`==`
      (set `self.BlockClick` false :!label _label_3))
    (:`<`
      (goto _label_3)))
  (`KismetSystemLibrary.Delay` 0.5)
  (set `self.Show player hand value` true))

(event `StartGame`
  (bind _deck (`self.Deck`))
  (bind _returnvalue (* (`self.NoOfDecks`) 4))
  ;[1 1 1] New game
  (`/Game/Blueprints/BP_Deck.InitializeDeck` _deck _returnvalue 13)
  (`/Game/Blueprints/BP_Deck.ShuffleDeck` _deck)
  (set `self.PlayersCash` 100.0)
  (set `self.Total Number of Cards` (* _returnvalue 13))
  (set `self.Index` 0)
  (set `self.GameEnded` false)
  (set `self.BlockClick` false)
  (`KismetSystemLibrary.Delay` 1.0)
  (`/Game/Blueprints/BP_Buttons.UIMode` (`self.Buttons`) (`self.CashPool`) (`self.PlayersCash`) "ShowBetAmounts" :!label _label_4))

(event `NextRound`
  ;[1 1 1] Main control
  (set `self.BlockClick` false)
  (goto _label_4))

(event `STAND`
  (bind _ai_hand_value (`self.AI Hand Value`))
  ;[1 1 1] Show Ai Hand
  (set `self.BlockClick` true)
  (bind _asbp_card_c (cast `/Game/Blueprints/BP_Card` (`KismetArrayLibrary.Array_Get` (`self.AI Cards in Hand`))))
  (`/Game/Blueprints/BP_Card.Rotate` _asbp_card_c)
  (set `self.Show AI hand value` true :!label _label_5)
  (`/Engine/EditorBlueprintResources/StandardMacros.CompareInt` _ai_hand_value 17 :!label _label_6
    (:`>`
      (`/Engine/EditorBlueprintResources/StandardMacros.CompareInt` _ai_hand_value 21
        (:`>`
          ;;[1 1 1] Check if AI have ace
          (`/Engine/EditorBlueprintResources/StandardMacros.CompareInt` (`self.AI Hand Aces`)
            (:`>`
              (set `self.AI Hand Value` (- (`self.AI Hand Value`) 10))
              (set `self.AI Hand Aces` (- (`self.AI Hand Aces`) 1))
              (goto _label_6))
            (:`==`
              (`self.AIOver21points`))))
        (:`==`
          (`self.Compare` :!label _label_7))
        (:`<`
          (goto _label_7))))
    (:`==`
      (goto _label_7))
    (:`<`
      (`KismetSystemLibrary.Delay` 1.0)
      (`self.AIDrawOneMoreCard`)))
  (`KismetSystemLibrary.Delay` 0.5)
  (set `self.Show player hand value` true))

(event `Reset`
  ;[1 1 1] Reset variables for new round
  (set `self.No of cards in hand` 0)
  (set `self.AI No of cards in hand` 0)
  (set `self.PlayersHandValue` 0)
  (set `self.AI Hand Value` 0)
  (set `self.Player hand aces` 0)
  (set `self.AI Hand Aces` 0)
  (set `self.CardIndexInHand` 0)
  (set `self.AI Card Index in Hand` 0)
  (`KismetArrayLibrary.Array_Clear` (`self.CardsInHand`))
  (`KismetArrayLibrary.Array_Clear` (`self.AI Cards in Hand`))
  (set `self.Show player hand value` false)
  (set `self.Show AI hand value` false))

(event `AIDrawOneMoreCard`
  (bind _ai_card_x_location (`self.AI Card x location`))
  (bind _ai_no_of_cards_in_hand (`self.AI No of cards in hand`))
  ;[1 1 1] AI Cards Placing
  (`|ExecutionSequence`
    (:`then_0`
      (switch `int` _ai_no_of_cards_in_hand :!label _label_8
        (:`0`
          (set `self.AI Card x location` -50.0)
          (set `self.AutoRotate` false))
        (:`1`
          (set `self.AI Card x location` (* (+ (`KismetMathLibrary.Abs` _ai_card_x_location) (* 1 110.0)) (* (`KismetMathLibrary.FClamp` _ai_card_x_location -1.0) -1.0)) :!label _label_9)
          (set `self.AutoRotate` true))
        (:`2`
          (goto _label_9))
        (:`3`
          (goto _label_9))
        (:`4`
          (goto _label_9))
        (:`5`
          (goto _label_9))
        (:`6`
          (goto _label_9))
        (:`7`
          (goto _label_9))
        (:`8`
          (goto _label_9)))
      (set `self.AI No of cards in hand` (+ _ai_no_of_cards_in_hand 1))
      (set `self.CardID` (`KismetArrayLibrary.Array_Get` (`self.Card Deck Shuffled`) (`self.Index`)))
      (bind _returnvalue (`|SpawnActorFromClass` "/Game/Blueprints/BP_Card.BP_Card_C" (`KismetMathLibrary.Conv_VectorToTransform` (`KismetMathLibrary.MakeVector` _ai_card_x_location 100.0 20.0))))
      (set `/Game/Blueprints/BP_Card.AutoRotate` (`self.AutoRotate`) _returnvalue)
      (set `/Game/Blueprints/BP_Card.LogicForCard` self _returnvalue)
      (`/Game/Blueprints/BP_Card.SetupCardID` _returnvalue (`self.CardID`))
      ;[1 1 1] Calculate AI hand
      (set `self.Index` (+ (`self.Index`) 1))
      (`KismetArrayLibrary.Array_Add` (`self.AI Cards in Hand`) _returnvalue)
      (set `self.AI Card Index in Hand` (+ (`self.AI Card Index in Hand`) 1))
      (bind (_cardvalue _ace) (`self.CalculateCardvalue` (`self.CardID`)))
      (if _ace
        (set `self.AI Hand Aces` (+ (`self.AI Hand Aces`) 1)))
      (set `self.AI Hand Value` (+ _cardvalue (`self.AI Hand Value`))))
    (:`then_1`
      (`self.CheckAIHand`))))

(event `CheckAIHand`
  ;[1 1 1] Show Ai Hand
  (goto _label_5))

(event `Click_HIT`
  ;[1 1 1] Main control
  (if (`self.GameEnded`)
    _
    (elif (not (`self.BlockClick`))
      (`ActorComponent.Activate` (`/Game/Blueprints/BP_Buttons.Left button effect` (`self.Buttons`)) false)
      (set `self.BlockClick` true :!label _label_10)
      (`self.Create Card`))))

(event `AIDrawInitialCards`
  ;[1 1 1] AI Cards Placing
  (`|ExecutionSequence`
    (:`then_0`
      (goto _label_8))
    (:`then_1`
      (goto _label_8))))

(event `Click_STAND`
  ;[1 1 1] Main control
  (if (`self.GameEnded`)
    _
    (elif (not (`self.BlockClick`))
      (`ActorComponent.Activate` (`/Game/Blueprints/BP_Buttons.Middle button effect` (`self.Buttons`)) false)
      (`GameplayStatics.PlaySoundAtLocation` "/Game/Assets/Sounds/ChipPush_Stereo_Cue.ChipPush_Stereo_Cue")
      (`self.STAND`))))

(event `Click_DOUBLE`
  ;[1 1 1] Main control
  (if (`self.GameEnded`)
    _
    (elif (not (`self.BlockClick`))
      (`ActorComponent.Activate` (`/Game/Blueprints/BP_Buttons.Right button effect` (`self.Buttons`)) false)
      (`GameplayStatics.PlaySoundAtLocation` "/Game/Assets/Sounds/ChipPush_Stereo_Cue.ChipPush_Stereo_Cue")
      (`|ExecutionSequence`
        (:`then_0`
          (`self.UpdateCountersDOUBLE`))
        (:`then_1`
          (goto _label_10))
        (:`then_2`
          (`/Game/Blueprints/BP_Buttons.UIMode` (`self.Buttons`) (`self.CashPool`) (`self.PlayersCash`) "HideStand"))))))

(event `Click_butt_5`
  ;[1 1 1] Stake selecting
  (if (not (`self.BlockClick`))
    (set `self.InitialStake` 5.0)
    (`ActorComponent.Activate` (`/Game/Blueprints/BP_Buttons.Left button effect` (`self.Buttons`)) false)
    (`self.UpdateCounters` :!label _label_11)
    (`GameplayStatics.PlaySoundAtLocation` "/Game/Assets/Sounds/ChipPush_Stereo_Cue.ChipPush_Stereo_Cue")
    (`/Game/Blueprints/BP_Buttons.UIMode` (`self.Buttons`) (`self.CashPool`) (`self.PlayersCash`) "ShowBettingOptions")
    (`|ExecutionSequence`
      (:`then_0`
        (set `self.BlockClick` true))
      (:`then_1`
        (`self.Create Card` :!label _label_12))
      (:`then_2`
        (goto _label_12))
      (:`then_3`
        (`self.AIDrawInitialCards`))
      (:`then_4`
        (`/Game/Blueprints/BP_Buttons.UIMode` (`self.Buttons`) (`self.CashPool`) (`self.PlayersCash`) "HideStand")))))

(event `Click_butt_10`
  ;[1 1 1] Stake selecting
  (if (not (`self.BlockClick`))
    (set `self.InitialStake` 10.0)
    (`ActorComponent.Activate` (`/Game/Blueprints/BP_Buttons.Middle button effect` (`self.Buttons`)) false)
    (goto _label_11)))

(event `Click_butt_25`
  ;[1 1 1] Stake selecting
  (if (not (`self.BlockClick`))
    (set `self.InitialStake` 25.0)
    (`ActorComponent.Activate` (`/Game/Blueprints/BP_Buttons.Right button effect` (`self.Buttons`)) false)
    (goto _label_11)))

(event `PlayerOver21points`
  ;[1 1 1] Show info when over 21 pts
  (set `self.BlockClick` true)
  (`KismetSystemLibrary.Delay` 0.5)
  (`self.UpdateHud` 0)
  ;[1 1 1] Lost - over 21 ot in hand
  (`KismetSystemLibrary.Delay` 2.0)
  (`self.GameLost`)
  (`self.ClearTable`)
  (`self.CheckRoundEnd`))

(event `AIOver21points`
  ;[1 1 1] Show info when over 21 pts
  (`KismetSystemLibrary.Delay` 0.5)
  (`self.UpdateHud` 4)
  ;[1 1 1] Update Cash on win
  (`KismetSystemLibrary.Delay` 2.0 :!label _label)
  (set `self.PlayersCash` (+ (`self.PlayersCash`) (`self.CashPool`)))
  (set `self.CashPool` 0.0)
  (`self.ClearTable`)
  (`self.CheckRoundEnd`))

(event `ClearTable`
  ;[1 1 1] Clear table
  (for _array_element (`self.CardsInHand`)
    (`self.K2_DestroyActor` _array_element))
  (for _array_element_2 (`self.AI Cards in Hand`)
    (`self.K2_DestroyActor` _array_element_2))
  (`self.Reset`))

(event `Compare`
  ;[1 1 1] Check who has better hand
  (`KismetSystemLibrary.Delay` 0.5)
  (`/Engine/EditorBlueprintResources/StandardMacros.CompareInt` (`self.PlayersHandValue`) (`self.AI Hand Value`)
    (:`>`
      (`self.UpdateHud` 2)
      (goto _label))
    (:`==`
      (`self.UpdateHud` 3)
      ;[1 1 1] Update cash on Draw
      (`KismetSystemLibrary.Delay` 2.0)
      (set `self.PlayersCash` (+ (`self.PlayersCash`) (/ (`self.CashPool`) 2.0)))
      (set `self.CashPool` 0.0)
      (`self.ClearTable`)
      (`self.CheckRoundEnd`))
    (:`<`
      (`self.UpdateHud` 1)
      ;[1 1 1] Update on loss
      (`KismetSystemLibrary.Delay` 2.0)
      (set `self.CashPool` 0.0 :!label _label_2)
      (`self.ClearTable`)
      (`self.CheckRoundEnd`))))

(event `CheckRoundEnd`
  ;[1 1 1] Check if next round can be played
  (`|ExecutionSequence`
    (:`then_0`
      (`/Engine/EditorBlueprintResources/StandardMacros.CompareFloat` (`self.PlayersCash`) 5.0
        (:`<`
          (`self.Bankrupt`))))
    (:`then_1`
      (switch `int` (`self.NoOfDecks`)
        (:`1`
          (set `self.MinCardsNeeded` 17))
        (:`3`
          (set `self.MinCardsNeeded` 27))
        (:`5`
          (set `self.MinCardsNeeded` 32))
        (:`7`
          (set `self.MinCardsNeeded` 36))))
    (:`then_2`
      (`/Engine/EditorBlueprintResources/StandardMacros.CompareInt` (`self.Index`) (- (`self.Total Number of Cards`) (`self.MinCardsNeeded`))
        (:`>`
          (`KismetSystemLibrary.Delay` 1.0)
          (`self.DeckEnd`))
        (:`==`
          (`self.NextRound` :!label _label_3))
        (:`<`
          (goto _label_3))))))

(event `GameLost`
  ;[1 1 1] Update on loss
  (goto _label_2))

(event `Bankrupt`
  ;[1 1 1] Bankrupt info
  (`self.UpdateHud` 5)
  (set `self.GameEnded` true)
  (`KismetSystemLibrary.Delay` 3.0)
  (`/Game/Blueprints/BP_Menu.NewGame` (`self.Menu`) :!label _label_4)
  (`self.ClearTable`))

(event `DeckEnd`
  ;[1 1 1] Deck End
  (`self.UpdateHud` 6)
  (set `self.GameEnded` true)
  (`KismetSystemLibrary.Delay` 3.0)
  (goto _label_4))

(event `UpdateCounters`
  ;[1 1 1] Update Cash and Pool
  (set `self.PlayersCash` (- (`self.PlayersCash`) (`self.InitialStake`)))
  (set `self.CashPool` (+ (`self.CashPool`) (* (`self.InitialStake`) 2.0))))

(event `UpdateCountersDOUBLE`
  (bind _cashpool (`self.CashPool`))
  ;[1 1 1] Update Cash and Pool when DOUBLE
  (set `self.PlayersCash` (+ (`self.PlayersCash`) (* _cashpool -0.5)))
  (set `self.CashPool` (* _cashpool 2.0)))

(fn `CalculateCardvalue`
  (params (CardID :type Integer))
  (returns (CardValue :type Integer) (Ace :type Boolean))
  (bind _currentcardid (`self.CurrentCardID`))
  (bind _returnvalue (- _currentcardid (* (/ _currentcardid 52) 52)))
  (bind _returnvalue_2 (- _returnvalue (* (/ _returnvalue 13) 13)))
  ;[1 1 1] Decode card ID
  (set `self.CurrentCardID` CardID)
  (`|ExecutionSequence`
    (:`then_0`
      ;[1 1 1] Set value
      (switch `int` _returnvalue_2
        (:`0`
          (set `self.CardValue` (+ _returnvalue_2 2) :!label _label)
          (set `self.Ace` false :!label _label_2))
        (:`1`
          (goto _label))
        (:`2`
          (goto _label))
        (:`3`
          (goto _label))
        (:`4`
          (goto _label))
        (:`5`
          (goto _label))
        (:`6`
          (goto _label))
        (:`7`
          (goto _label))
        (:`8`
          (goto _label))
        (:`9`
          (set `self.CardValue` 10 :!label _label_3)
          (goto _label_2))
        (:`10`
          (goto _label_3))
        (:`11`
          (goto _label_3))
        (:`12`
          (set `self.CardValue` 11)
          (set `self.Ace` true)))
      (return (`self.CardValue`) (`self.Ace`)))))

(fn `UpdateHud`
  (params (InOption :type Integer))
  (bind _asbp_hud_bj_c (cast `/Game/Blueprints/BP_HUD_BJ` (`PlayerController.GetHUD` (`GameplayStatics.GetPlayerController` 0))))
  (`/Game/Blueprints/BP_HUD_BJ.UpdateHud` _asbp_hud_bj_c InOption))

(fn `UserConstructionScript`
  ;[1 1 1] Initial setup
  (set `self.NoOfDecks` 5))