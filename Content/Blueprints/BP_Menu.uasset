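; BP_Menu is the in-world game menu that slides into view for a new game and away when play starts.
; On BeginPlay it caches the BP_Logic game mode and runs NewGame, which shows MenuRoot, plays the right Matinee and follows with a delayed sound.
; Clicking or touching PlayButton plays the left Matinee, calls StartGame on BP_Logic with a sound, then hides MenuRoot after a short delay.
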(event `self.ReceiveBeginPlay`
  ;[1 1 1] Initialise
  (bind _asbp_logic_c (cast `/Game/Blueprints/BP_Logic` (`GameplayStatics.GetGameMode`)))
  (set `self.Logic` _asbp_logic_c)
  (`self.NewGame`))

(event `NewGame`
  ;[1 1 1] Set initial menu position
  (`SceneComponent.SetVisibility` (`self.MenuRoot`) true true)
  (bind _asmatineeactor (cast `MatineeActor` (`self.Matinee-MenuRight`)))
  (`MatineeActor.Play` _asmatineeactor)
  (`KismetSystemLibrary.Delay` 0.5)
  ;;[1 1 1] Sound Continue
  (`GameplayStatics.PlaySoundAtLocation` "/Game/Assets/Sounds/Frontend_Continue_Stereo_Cue.Frontend_Continue_Stereo_Cue"))

(event `self.Play button.OnClicked`
  (params (TouchedComponent :type "PrimitiveComponent Object Reference"))
  ;[1 1 1] Send menu to hidden possition
  (bind _asmatineeactor (cast `MatineeActor` (`self.Matinee-Menu Left`) :!label _label))
  (`MatineeActor.Play` _asmatineeactor)
  (`/Game/Blueprints/BP_Logic.StartGame` (`self.Logic`))
  ;;[1 1 1] Sound Continue
  (`GameplayStatics.PlaySoundAtLocation` "/Game/Assets/Sounds/Frontend_Continue_Stereo_Cue.Frontend_Continue_Stereo_Cue")
  (`KismetSystemLibrary.Delay` 0.7)
  (`SceneComponent.SetVisibility` (`self.MenuRoot`) false false))

(event `self.Play button.OnInputTouchBegin`
  (params (FingerIndex :type "InputCoreTypes.ETouchIndex Enum" :default "Touch1") (TouchedComponent :type "PrimitiveComponent Object Reference"))
  ;[1 1 1] Send menu to hidden possition
  (goto _label))

(fn `UserConstructionScript`)