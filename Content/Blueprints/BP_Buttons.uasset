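; Clickable 3D button set for a blackjack-style game: Hit, Stand, Double and three bet amounts.
; Buttons rise on hover and forward clicks or touches to the BP_Logic game mode, with Hit also activating an effect.
; UIMode toggles visibility and collision between action and bet buttons, revealing affordable bets and hiding Double when player cash is below half the pool.
; ClickEffect spawns a pulse ring unless clicks are blocked, but is not called here.
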(event `self.ReceiveBeginPlay`
  ;[1 1 1] Initialise
  (bind _asbp_logic_c (cast `/Game/Blueprints/BP_Logic` (`GameplayStatics.GetGameMode`)))
  (set `self.Logic` _asbp_logic_c))

(event `self.Button HIT.OnBeginCursorOver`
  (params (TouchedComponent :type "PrimitiveComponent Object Reference"))
  ;[1 1 1] Cursor Over Button effects
  (set `self.Location` (0.0 0.0 10.0))
  (`SceneComponent.AddLocalOffset` (`self.Button HIT`) (`self.Location`) false :!label _label))

(event `self.Button HIT.OnEndCursorOver`
  (params (TouchedComponent :type "PrimitiveComponent Object Reference"))
  ;[1 1 1] Cursor Over Button effects
  (set `self.Location` (0.0 0.0 -10.0))
  (goto _label))

(event `self.Button STAND.OnBeginCursorOver`
  (params (TouchedComponent :type "PrimitiveComponent Object Reference"))
  ;[1 1 1] Cursor Over Button effects
  (set `self.Location` (0.0 0.0 10.0))
  (`SceneComponent.AddLocalOffset` (`self.Button STAND`) (`self.Location`) false :!label _label_2))

(event `self.Button STAND.OnEndCursorOver`
  (params (TouchedComponent :type "PrimitiveComponent Object Reference"))
  ;[1 1 1] Cursor Over Button effects
  (set `self.Location` (0.0 0.0 -10.0))
  (goto _label_2))

(event `self.Button HIT.OnClicked`
  (params (TouchedComponent :type "PrimitiveComponent Object Reference"))
  ;[1 1 1] Onclick activation for buttons
  (`/Game/Blueprints/BP_Logic.Click_HIT` (`self.Logic`) :!label _label_3)
  (`ActorComponent.Activate` (`self.Left button effect`) false))

(event `self.Button DOUBLE STAND.OnBeginCursorOver`
  (params (TouchedComponent :type "PrimitiveComponent Object Reference"))
  ;[1 1 1] Cursor Over Button effects
  (set `self.Location` (0.0 0.0 10.0))
  (`SceneComponent.AddLocalOffset` (`self.Button DOUBLE STAND`) (`self.Location`) false :!label _label_4))

(event `self.Button HIT.OnInputTouchBegin`
  (params (FingerIndex :type "InputCoreTypes.ETouchIndex Enum" :default "Touch1") (TouchedComponent :type "PrimitiveComponent Object Reference"))
  ;[1 1 1] Onclick activation for buttons
  (goto _label_3))

(event `self.Button DOUBLE STAND.OnEndCursorOver`
  (params (TouchedComponent :type "PrimitiveComponent Object Reference"))
  ;[1 1 1] Cursor Over Button effects
  (set `self.Location` (0.0 0.0 -10.0))
  (goto _label_4))

(event `self.Button STAND.OnClicked`
  (params (TouchedComponent :type "PrimitiveComponent Object Reference"))
  ;[1 1 1] Onclick activation for buttons
  (`/Game/Blueprints/BP_Logic.Click_STAND` (`self.Logic`) :!label _label_5))

(event `self.Button STAND.OnInputTouchBegin`
  (params (FingerIndex :type "InputCoreTypes.ETouchIndex Enum" :default "Touch1") (TouchedComponent :type "PrimitiveComponent Object Reference"))
  ;[1 1 1] Onclick activation for buttons
  (goto _label_5))

(event `self.Button 5.OnBeginCursorOver`
  (params (TouchedComponent :type "PrimitiveComponent Object Reference"))
  ;[1 1 1] Cursor Over Button effects
  (set `self.Location` (0.0 0.0 10.0))
  (`SceneComponent.AddLocalOffset` (`self.Button 5`) (`self.Location`) false :!label _label_6))

(event `self.Button DOUBLE STAND.OnClicked`
  (params (TouchedComponent :type "PrimitiveComponent Object Reference"))
  ;[1 1 1] Onclick activation for buttons
  (`/Game/Blueprints/BP_Logic.Click_DOUBLE` (`self.Logic`) :!label _label_7))

(event `self.Button DOUBLE STAND.OnInputTouchBegin`
  (params (FingerIndex :type "InputCoreTypes.ETouchIndex Enum" :default "Touch1") (TouchedComponent :type "PrimitiveComponent Object Reference"))
  ;[1 1 1] Onclick activation for buttons
  (goto _label_7))

(event `self.Button 5.OnEndCursorOver`
  (params (TouchedComponent :type "PrimitiveComponent Object Reference"))
  ;[1 1 1] Cursor Over Button effects
  (set `self.Location` (0.0 0.0 -10.0))
  (goto _label_6))

(event `self.Button 5.OnClicked`
  (params (TouchedComponent :type "PrimitiveComponent Object Reference"))
  ;[1 1 1] Onclick activation for buttons
  (`/Game/Blueprints/BP_Logic.Click_butt_5` (`self.Logic`) :!label _label_8))

(event `self.Button 10.OnBeginCursorOver`
  (params (TouchedComponent :type "PrimitiveComponent Object Reference"))
  ;[1 1 1] Cursor Over Button effects
  (set `self.Location` (0.0 0.0 10.0))
  (`SceneComponent.AddLocalOffset` (`self.Button 10`) (`self.Location`) false :!label _label_9))

(event `self.Button 5.OnInputTouchBegin`
  (params (FingerIndex :type "InputCoreTypes.ETouchIndex Enum" :default "Touch1") (TouchedComponent :type "PrimitiveComponent Object Reference"))
  ;[1 1 1] Onclick activation for buttons
  (goto _label_8))

(event `self.Button 10.OnEndCursorOver`
  (params (TouchedComponent :type "PrimitiveComponent Object Reference"))
  ;[1 1 1] Cursor Over Button effects
  (set `self.Location` (0.0 0.0 -10.0))
  (goto _label_9))

(event `self.Button 10.OnClicked`
  (params (TouchedComponent :type "PrimitiveComponent Object Reference"))
  ;[1 1 1] Onclick activation for buttons
  (`/Game/Blueprints/BP_Logic.Click_butt_10` (`self.Logic`) :!label _label_10))

(event `self.Button 10.OnInputTouchBegin`
  (params (FingerIndex :type "InputCoreTypes.ETouchIndex Enum" :default "Touch1") (TouchedComponent :type "PrimitiveComponent Object Reference"))
  ;[1 1 1] Onclick activation for buttons
  (goto _label_10))

(event `self.Button 25.OnBeginCursorOver`
  (params (TouchedComponent :type "PrimitiveComponent Object Reference"))
  ;[1 1 1] Cursor Over Button effects
  (set `self.Location` (0.0 0.0 10.0))
  (`SceneComponent.AddLocalOffset` (`self.Button 25`) (`self.Location`) false :!label _label_11))

(event `self.Button 25.OnClicked`
  (params (TouchedComponent :type "PrimitiveComponent Object Reference"))
  ;[1 1 1] Onclick activation for buttons
  (`/Game/Blueprints/BP_Logic.Click_butt_25` (`self.Logic`) :!label _label_12))

(event `self.Button 25.OnInputTouchBegin`
  (params (FingerIndex :type "InputCoreTypes.ETouchIndex Enum" :default "Touch1") (TouchedComponent :type "PrimitiveComponent Object Reference"))
  ;[1 1 1] Onclick activation for buttons
  (goto _label_12))

(event `self.Button 25.OnEndCursorOver`
  (params (TouchedComponent :type "PrimitiveComponent Object Reference"))
  ;[1 1 1] Cursor Over Button effects
  (set `self.Location` (0.0 0.0 -10.0))
  (goto _label_11))

(event `UIMode`
  (params (CashPool :type "Float (double-precision)") (PlayersCash :type "Float (double-precision)") (UIMode :type "/Game/Blueprints/UIMode Enum"))
  (bind _button_5 (`self.Button 5`))
  (bind _button_10 (`self.Button 10`))
  (bind _button_25 (`self.Button 25`))
  (bind _playerscash (`self.PlayersCash`))
  (bind _button_double_stand (`self.Button DOUBLE STAND`))
  ;[1 1 1] UI Mode Toggling
  (set `self.CashPool` CashPool)
  (set `self.PlayersCash` PlayersCash)
  (switch `/Game/Blueprints/UIMode` UIMode
    (:`ShowBettingOptions`
      (`SceneComponent.SetVisibility` _button_double_stand true true)
      (`SceneComponent.SetVisibility` (`self.Button STAND`) true true)
      (`SceneComponent.SetVisibility` (`self.Button HIT`) true true)
      (`PrimitiveComponent.SetCollisionEnabled` _button_double_stand "QueryAndPhysics")
      (`PrimitiveComponent.SetCollisionEnabled` (`self.Button STAND`) "QueryAndPhysics")
      (`PrimitiveComponent.SetCollisionEnabled` (`self.Button HIT`) "QueryAndPhysics")
      (`SceneComponent.SetVisibility` _button_25 false true)
      (`SceneComponent.SetVisibility` _button_10 false true)
      (`SceneComponent.SetVisibility` _button_5 false true)
      (`PrimitiveComponent.SetCollisionEnabled` _button_25 "NoCollision")
      (`PrimitiveComponent.SetCollisionEnabled` _button_10 "NoCollision")
      (`PrimitiveComponent.SetCollisionEnabled` _button_5 "NoCollision"))
    (:`ShowBetAmounts`
      (`SceneComponent.SetVisibility` _button_double_stand false true)
      (`SceneComponent.SetVisibility` (`self.Button STAND`) false true)
      (`SceneComponent.SetVisibility` (`self.Button HIT`) false true)
      (`PrimitiveComponent.SetCollisionEnabled` _button_double_stand "NoCollision")
      (`PrimitiveComponent.SetCollisionEnabled` (`self.Button STAND`) "NoCollision")
      (`PrimitiveComponent.SetCollisionEnabled` (`self.Button HIT`) "NoCollision")
      (`/Engine/EditorBlueprintResources/StandardMacros.CompareFloat` _playerscash 25.0
        (:`>`
          (`SceneComponent.SetVisibility` _button_25 true true :!label _label_13)
          (`PrimitiveComponent.SetCollisionEnabled` _button_25 "QueryAndPhysics"))
        (:`==`
          (goto _label_13))
        (:`<`
          _))
      (`/Engine/EditorBlueprintResources/StandardMacros.CompareFloat` _playerscash 10.0
        (:`>`
          (`SceneComponent.SetVisibility` _button_10 true true :!label _label_14)
          (`PrimitiveComponent.SetCollisionEnabled` _button_10 "QueryAndPhysics"))
        (:`==`
          (goto _label_14))
        (:`<`
          _))
      (`/Engine/EditorBlueprintResources/StandardMacros.CompareFloat` _playerscash 5.0
        (:`>`
          _)
        (:`==`
          _))
      (`SceneComponent.SetVisibility` _button_5 true true)
      (`PrimitiveComponent.SetCollisionEnabled` _button_5 "QueryAndPhysics"))
    (:`HideStand`
      (`/Engine/EditorBlueprintResources/StandardMacros.CompareFloat` (`self.PlayersCash`) (/ (`self.CashPool`) 2.0)
        (:`<`
          (`SceneComponent.SetVisibility` _button_double_stand false true)
          (`PrimitiveComponent.SetCollisionEnabled` _button_double_stand "NoCollision"))))))

(fn `Click effect`
  (params (Button :type "StaticMeshComponent Object Reference"))
  (if (not (`/Game/Blueprints/BP_Logic.BlockClick` (`self.Logic`)))
    (`GameplayStatics.SpawnEmitterAtLocation` "/Game/Assets/Effects/particles/P_Pulse_Ring.P_Pulse_Ring" (`KismetMathLibrary.MakeVector` (.x (`SceneComponent.K2_GetComponentLocation` Button)) (.y (`SceneComponent.K2_GetComponentLocation` Button))))))

(fn `UserConstructionScript`)