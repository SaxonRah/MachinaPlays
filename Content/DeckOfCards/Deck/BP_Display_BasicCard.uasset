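; Displays one playing card as a static mesh actor, textured to match its rank, suit and facing.
; The construction script and SetCard call SetupCardMaterials, which creates dynamic edge, back and face materials, swapping front/back slots by IsFaceUp.
; Nested switches set the "Card" texture, with UseFaceCards choosing alternate art for court cards and the Ace of Spades.
; Nine of Hearts uses the spades texture, as does alternate Jack of Spades the clubs one.
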(event EventBeginPlay)

(event Collision|EventActorBeginOverlap
  (params (OtherActor :type Actor%20Object%20Reference)))

(event EventTick
  (params (DeltaSeconds :type Float%20%28single-precision%29))
  (Variables|Default|SetWorldTransform (Variables|Default|GetWorldTransform)))

(fn ConstructionScript
  (CallFunction|SetupCardMaterials))

(fn SetCard
  (params (Card :type Standard%20Card%20Structure))
  (Variables|Default|SetThisCard Card)
  (CallFunction|SetupCardMaterials))

(fn SetupCardMaterials
  (bind _thiscard (Variables|Default|GetThisCard))
  (bind _staticmeshcomponent (Variables|Debug|GetStaticMeshComponent))
  (bind (_suit _rank) (Utilities|Struct|BreakStandardCard _thiscard))
  (Rendering|Material|CreateDynamicMaterialInstance _staticmeshcomponent 2 "/Game/DeckOfCards/Deck/Materials/M_CardEdge_Master.M_CardEdge_Master" :!class /Script/Engine.PrimitiveComponent)
  (if (Variables|Default|GetbIsFaceUp)
    (Rendering|Material|CreateDynamicMaterialInstance _staticmeshcomponent 1 "/Game/DeckOfCards/Deck/Materials/MI_BackOfCard.MI_BackOfCard" :!class /Script/Engine.PrimitiveComponent)
    (bind _returnvalue (Rendering|Material|CreateDynamicMaterialInstance _staticmeshcomponent 0 "/Game/DeckOfCards/Deck/Materials/M_Card_Master.M_Card_Master" :!class /Script/Engine.PrimitiveComponent))
    (Variables|Default|SetCard_MaterialInst _returnvalue)
    (else
      (Rendering|Material|CreateDynamicMaterialInstance _staticmeshcomponent 0 "/Game/DeckOfCards/Deck/Materials/MI_BackOfCard.MI_BackOfCard" :!class /Script/Engine.PrimitiveComponent)
      (bind _returnvalue_2 (Rendering|Material|CreateDynamicMaterialInstance _staticmeshcomponent 1 "/Game/DeckOfCards/Deck/Materials/M_Card_Master.M_Card_Master" :!class /Script/Engine.PrimitiveComponent))
      (Variables|Default|SetCard_MaterialInst _returnvalue_2)))
  (LocalVariables|SetLocal_Suit _suit)
  (switch Utilities|FlowControl|Switch|SwitchonEStandardCardRank _rank
    (:CR_Ace
      (switch Utilities|FlowControl|Switch|SwitchonEStandardCardSuit (LocalVariables|GetLocal_Suit)
        (:CS_Spades
          (if (Variables|Default|GetbUseFaceCards)
            (Rendering|Material|SetTextureParameterValue (Variables|Default|GetCard_MaterialInst) "Card" "/Game/DeckOfCards/Deck/Texture/ace_of_spades.ace_of_spades")
            (else
              (Rendering|Material|SetTextureParameterValue (Variables|Default|GetCard_MaterialInst) "Card" "/Game/DeckOfCards/Deck/Texture/ace_of_spades2.ace_of_spades2"))))
        (:CS_Hearts
          (Rendering|Material|SetTextureParameterValue (Variables|Default|GetCard_MaterialInst) "Card" "/Game/DeckOfCards/Deck/Texture/ace_of_hearts.ace_of_hearts"))
        (:CS_Clubs
          (Rendering|Material|SetTextureParameterValue (Variables|Default|GetCard_MaterialInst) "Card" "/Game/DeckOfCards/Deck/Texture/ace_of_clubs.ace_of_clubs"))
        (:CS_Diamonds
          (Rendering|Material|SetTextureParameterValue (Variables|Default|GetCard_MaterialInst) "Card" "/Game/DeckOfCards/Deck/Texture/ace_of_diamonds.ace_of_diamonds"))))
    (:CR_Two
      (switch Utilities|FlowControl|Switch|SwitchonEStandardCardSuit (LocalVariables|GetLocal_Suit)
        (:CS_Spades
          (Rendering|Material|SetTextureParameterValue (Variables|Default|GetCard_MaterialInst) "Card" "/Game/DeckOfCards/Deck/Texture/2_of_spades.2_of_spades"))
        (:CS_Hearts
          (Rendering|Material|SetTextureParameterValue (Variables|Default|GetCard_MaterialInst) "Card" "/Game/DeckOfCards/Deck/Texture/2_of_hearts.2_of_hearts"))
        (:CS_Clubs
          (Rendering|Material|SetTextureParameterValue (Variables|Default|GetCard_MaterialInst) "Card" "/Game/DeckOfCards/Deck/Texture/2_of_clubs.2_of_clubs"))
        (:CS_Diamonds
          (Rendering|Material|SetTextureParameterValue (Variables|Default|GetCard_MaterialInst) "Card" "/Game/DeckOfCards/Deck/Texture/2_of_diamonds.2_of_diamonds"))))
    (:CR_Three
      (switch Utilities|FlowControl|Switch|SwitchonEStandardCardSuit (LocalVariables|GetLocal_Suit)
        (:CS_Spades
          (Rendering|Material|SetTextureParameterValue (Variables|Default|GetCard_MaterialInst) "Card" "/Game/DeckOfCards/Deck/Texture/3_of_spades.3_of_spades"))
        (:CS_Hearts
          (Rendering|Material|SetTextureParameterValue (Variables|Default|GetCard_MaterialInst) "Card" "/Game/DeckOfCards/Deck/Texture/3_of_hearts.3_of_hearts"))
        (:CS_Clubs
          (Rendering|Material|SetTextureParameterValue (Variables|Default|GetCard_MaterialInst) "Card" "/Game/DeckOfCards/Deck/Texture/3_of_clubs.3_of_clubs"))
        (:CS_Diamonds
          (Rendering|Material|SetTextureParameterValue (Variables|Default|GetCard_MaterialInst) "Card" "/Game/DeckOfCards/Deck/Texture/3_of_diamonds.3_of_diamonds"))))
    (:CR_Four
      (switch Utilities|FlowControl|Switch|SwitchonEStandardCardSuit (LocalVariables|GetLocal_Suit)
        (:CS_Spades
          (Rendering|Material|SetTextureParameterValue (Variables|Default|GetCard_MaterialInst) "Card" "/Game/DeckOfCards/Deck/Texture/4_of_spades.4_of_spades"))
        (:CS_Hearts
          (Rendering|Material|SetTextureParameterValue (Variables|Default|GetCard_MaterialInst) "Card" "/Game/DeckOfCards/Deck/Texture/4_of_hearts.4_of_hearts"))
        (:CS_Clubs
          (Rendering|Material|SetTextureParameterValue (Variables|Default|GetCard_MaterialInst) "Card" "/Game/DeckOfCards/Deck/Texture/4_of_clubs.4_of_clubs"))
        (:CS_Diamonds
          (Rendering|Material|SetTextureParameterValue (Variables|Default|GetCard_MaterialInst) "Card" "/Game/DeckOfCards/Deck/Texture/4_of_diamonds.4_of_diamonds"))))
    (:CR_Five
      (switch Utilities|FlowControl|Switch|SwitchonEStandardCardSuit (LocalVariables|GetLocal_Suit)
        (:CS_Spades
          (Rendering|Material|SetTextureParameterValue (Variables|Default|GetCard_MaterialInst) "Card" "/Game/DeckOfCards/Deck/Texture/5_of_spades.5_of_spades"))
        (:CS_Hearts
          (Rendering|Material|SetTextureParameterValue (Variables|Default|GetCard_MaterialInst) "Card" "/Game/DeckOfCards/Deck/Texture/5_of_hearts.5_of_hearts"))
        (:CS_Clubs
          (Rendering|Material|SetTextureParameterValue (Variables|Default|GetCard_MaterialInst) "Card" "/Game/DeckOfCards/Deck/Texture/5_of_clubs.5_of_clubs"))
        (:CS_Diamonds
          (Rendering|Material|SetTextureParameterValue (Variables|Default|GetCard_MaterialInst) "Card" "/Game/DeckOfCards/Deck/Texture/5_of_diamonds.5_of_diamonds"))))
    (:CR_Six
      (switch Utilities|FlowControl|Switch|SwitchonEStandardCardSuit (LocalVariables|GetLocal_Suit)
        (:CS_Spades
          (Rendering|Material|SetTextureParameterValue (Variables|Default|GetCard_MaterialInst) "Card" "/Game/DeckOfCards/Deck/Texture/6_of_spades.6_of_spades"))
        (:CS_Hearts
          (Rendering|Material|SetTextureParameterValue (Variables|Default|GetCard_MaterialInst) "Card" "/Game/DeckOfCards/Deck/Texture/6_of_hearts.6_of_hearts"))
        (:CS_Clubs
          (Rendering|Material|SetTextureParameterValue (Variables|Default|GetCard_MaterialInst) "Card" "/Game/DeckOfCards/Deck/Texture/6_of_clubs.6_of_clubs"))
        (:CS_Diamonds
          (Rendering|Material|SetTextureParameterValue (Variables|Default|GetCard_MaterialInst) "Card" "/Game/DeckOfCards/Deck/Texture/6_of_diamonds.6_of_diamonds"))))
    (:CR_Seven
      (switch Utilities|FlowControl|Switch|SwitchonEStandardCardSuit (LocalVariables|GetLocal_Suit)
        (:CS_Spades
          (Rendering|Material|SetTextureParameterValue (Variables|Default|GetCard_MaterialInst) "Card" "/Game/DeckOfCards/Deck/Texture/7_of_spades.7_of_spades"))
        (:CS_Hearts
          (Rendering|Material|SetTextureParameterValue (Variables|Default|GetCard_MaterialInst) "Card" "/Game/DeckOfCards/Deck/Texture/7_of_hearts.7_of_hearts"))
        (:CS_Clubs
          (Rendering|Material|SetTextureParameterValue (Variables|Default|GetCard_MaterialInst) "Card" "/Game/DeckOfCards/Deck/Texture/7_of_clubs.7_of_clubs"))
        (:CS_Diamonds
          (Rendering|Material|SetTextureParameterValue (Variables|Default|GetCard_MaterialInst) "Card" "/Game/DeckOfCards/Deck/Texture/7_of_diamonds.7_of_diamonds"))))
    (:CR_Eight
      (switch Utilities|FlowControl|Switch|SwitchonEStandardCardSuit (LocalVariables|GetLocal_Suit)
        (:CS_Spades
          (Rendering|Material|SetTextureParameterValue (Variables|Default|GetCard_MaterialInst) "Card" "/Game/DeckOfCards/Deck/Texture/8_of_spades.8_of_spades"))
        (:CS_Hearts
          (Rendering|Material|SetTextureParameterValue (Variables|Default|GetCard_MaterialInst) "Card" "/Game/DeckOfCards/Deck/Texture/8_of_hearts.8_of_hearts"))
        (:CS_Clubs
          (Rendering|Material|SetTextureParameterValue (Variables|Default|GetCard_MaterialInst) "Card" "/Game/DeckOfCards/Deck/Texture/8_of_clubs.8_of_clubs"))
        (:CS_Diamonds
          (Rendering|Material|SetTextureParameterValue (Variables|Default|GetCard_MaterialInst) "Card" "/Game/DeckOfCards/Deck/Texture/8_of_diamonds.8_of_diamonds"))))
    (:CR_Nine
      (switch Utilities|FlowControl|Switch|SwitchonEStandardCardSuit (LocalVariables|GetLocal_Suit)
        (:CS_Spades
          (Rendering|Material|SetTextureParameterValue (Variables|Default|GetCard_MaterialInst) "Card" "/Game/DeckOfCards/Deck/Texture/9_of_spades.9_of_spades"))
        (:CS_Hearts
          (Rendering|Material|SetTextureParameterValue (Variables|Default|GetCard_MaterialInst) "Card" "/Game/DeckOfCards/Deck/Texture/9_of_spades.9_of_spades"))
        (:CS_Clubs
          (Rendering|Material|SetTextureParameterValue (Variables|Default|GetCard_MaterialInst) "Card" "/Game/DeckOfCards/Deck/Texture/9_of_clubs.9_of_clubs"))
        (:CS_Diamonds
          (Rendering|Material|SetTextureParameterValue (Variables|Default|GetCard_MaterialInst) "Card" "/Game/DeckOfCards/Deck/Texture/9_of_diamonds.9_of_diamonds"))))
    (:CR_Ten
      (switch Utilities|FlowControl|Switch|SwitchonEStandardCardSuit (LocalVariables|GetLocal_Suit)
        (:CS_Spades
          (Rendering|Material|SetTextureParameterValue (Variables|Default|GetCard_MaterialInst) "Card" "/Game/DeckOfCards/Deck/Texture/10_of_spades.10_of_spades"))
        (:CS_Hearts
          (Rendering|Material|SetTextureParameterValue (Variables|Default|GetCard_MaterialInst) "Card" "/Game/DeckOfCards/Deck/Texture/10_of_hearts.10_of_hearts"))
        (:CS_Clubs
          (Rendering|Material|SetTextureParameterValue (Variables|Default|GetCard_MaterialInst) "Card" "/Game/DeckOfCards/Deck/Texture/10_of_clubs.10_of_clubs"))
        (:CS_Diamonds
          (Rendering|Material|SetTextureParameterValue (Variables|Default|GetCard_MaterialInst) "Card" "/Game/DeckOfCards/Deck/Texture/10_of_diamonds.10_of_diamonds"))))
    (:CR_Jack
      (if (Variables|Default|GetbUseFaceCards)
        (switch Utilities|FlowControl|Switch|SwitchonEStandardCardSuit (LocalVariables|GetLocal_Suit)
          (:CS_Spades
            (Rendering|Material|SetTextureParameterValue (Variables|Default|GetCard_MaterialInst) "Card" "/Game/DeckOfCards/Deck/Texture/jack_of_clubs2.jack_of_clubs2"))
          (:CS_Hearts
            (Rendering|Material|SetTextureParameterValue (Variables|Default|GetCard_MaterialInst) "Card" "/Game/DeckOfCards/Deck/Texture/jack_of_hearts2.jack_of_hearts2"))
          (:CS_Clubs
            (Rendering|Material|SetTextureParameterValue (Variables|Default|GetCard_MaterialInst) "Card" "/Game/DeckOfCards/Deck/Texture/jack_of_clubs2.jack_of_clubs2"))
          (:CS_Diamonds
            (Rendering|Material|SetTextureParameterValue (Variables|Default|GetCard_MaterialInst) "Card" "/Game/DeckOfCards/Deck/Texture/jack_of_diamonds2.jack_of_diamonds2")))
        (else
          (switch Utilities|FlowControl|Switch|SwitchonEStandardCardSuit (LocalVariables|GetLocal_Suit)
            (:CS_Spades
              (Rendering|Material|SetTextureParameterValue (Variables|Default|GetCard_MaterialInst) "Card" "/Game/DeckOfCards/Deck/Texture/jack_of_spades.jack_of_spades"))
            (:CS_Hearts
              (Rendering|Material|SetTextureParameterValue (Variables|Default|GetCard_MaterialInst) "Card" "/Game/DeckOfCards/Deck/Texture/jack_of_hearts.jack_of_hearts"))
            (:CS_Clubs
              (Rendering|Material|SetTextureParameterValue (Variables|Default|GetCard_MaterialInst) "Card" "/Game/DeckOfCards/Deck/Texture/jack_of_clubs.jack_of_clubs"))
            (:CS_Diamonds
              (Rendering|Material|SetTextureParameterValue (Variables|Default|GetCard_MaterialInst) "Card" "/Game/DeckOfCards/Deck/Texture/jack_of_diamonds.jack_of_diamonds"))))))
    (:CR_Queen
      (if (Variables|Default|GetbUseFaceCards)
        (switch Utilities|FlowControl|Switch|SwitchonEStandardCardSuit (LocalVariables|GetLocal_Suit)
          (:CS_Spades
            (Rendering|Material|SetTextureParameterValue (Variables|Default|GetCard_MaterialInst) "Card" "/Game/DeckOfCards/Deck/Texture/queen_of_spades2.queen_of_spades2"))
          (:CS_Hearts
            (Rendering|Material|SetTextureParameterValue (Variables|Default|GetCard_MaterialInst) "Card" "/Game/DeckOfCards/Deck/Texture/queen_of_hearts2.queen_of_hearts2"))
          (:CS_Clubs
            (Rendering|Material|SetTextureParameterValue (Variables|Default|GetCard_MaterialInst) "Card" "/Game/DeckOfCards/Deck/Texture/queen_of_clubs2.queen_of_clubs2"))
          (:CS_Diamonds
            (Rendering|Material|SetTextureParameterValue (Variables|Default|GetCard_MaterialInst) "Card" "/Game/DeckOfCards/Deck/Texture/queen_of_diamonds2.queen_of_diamonds2")))
        (else
          (switch Utilities|FlowControl|Switch|SwitchonEStandardCardSuit (LocalVariables|GetLocal_Suit)
            (:CS_Spades
              (Rendering|Material|SetTextureParameterValue (Variables|Default|GetCard_MaterialInst) "Card" "/Game/DeckOfCards/Deck/Texture/queen_of_spades.queen_of_spades"))
            (:CS_Hearts
              (Rendering|Material|SetTextureParameterValue (Variables|Default|GetCard_MaterialInst) "Card" "/Game/DeckOfCards/Deck/Texture/queen_of_hearts.queen_of_hearts"))
            (:CS_Clubs
              (Rendering|Material|SetTextureParameterValue (Variables|Default|GetCard_MaterialInst) "Card" "/Game/DeckOfCards/Deck/Texture/queen_of_clubs.queen_of_clubs"))
            (:CS_Diamonds
              (Rendering|Material|SetTextureParameterValue (Variables|Default|GetCard_MaterialInst) "Card" "/Game/DeckOfCards/Deck/Texture/queen_of_diamonds.queen_of_diamonds"))))))
    (:CR_King
      (if (Variables|Default|GetbUseFaceCards)
        (switch Utilities|FlowControl|Switch|SwitchonEStandardCardSuit (LocalVariables|GetLocal_Suit)
          (:CS_Spades
            (Rendering|Material|SetTextureParameterValue (Variables|Default|GetCard_MaterialInst) "Card" "/Game/DeckOfCards/Deck/Texture/king_of_spades2.king_of_spades2"))
          (:CS_Hearts
            (Rendering|Material|SetTextureParameterValue (Variables|Default|GetCard_MaterialInst) "Card" "/Game/DeckOfCards/Deck/Texture/king_of_hearts2.king_of_hearts2"))
          (:CS_Clubs
            (Rendering|Material|SetTextureParameterValue (Variables|Default|GetCard_MaterialInst) "Card" "/Game/DeckOfCards/Deck/Texture/king_of_clubs2.king_of_clubs2"))
          (:CS_Diamonds
            (Rendering|Material|SetTextureParameterValue (Variables|Default|GetCard_MaterialInst) "Card" "/Game/DeckOfCards/Deck/Texture/king_of_diamonds2.king_of_diamonds2")))
        (else
          (switch Utilities|FlowControl|Switch|SwitchonEStandardCardSuit (LocalVariables|GetLocal_Suit)
            (:CS_Spades
              (Rendering|Material|SetTextureParameterValue (Variables|Default|GetCard_MaterialInst) "Card" "/Game/DeckOfCards/Deck/Texture/king_of_spades.king_of_spades"))
            (:CS_Hearts
              (Rendering|Material|SetTextureParameterValue (Variables|Default|GetCard_MaterialInst) "Card" "/Game/DeckOfCards/Deck/Texture/king_of_hearts.king_of_hearts"))
            (:CS_Clubs
              (Rendering|Material|SetTextureParameterValue (Variables|Default|GetCard_MaterialInst) "Card" "/Game/DeckOfCards/Deck/Texture/king_of_clubs.king_of_clubs"))
            (:CS_Diamonds
              (Rendering|Material|SetTextureParameterValue (Variables|Default|GetCard_MaterialInst) "Card" "/Game/DeckOfCards/Deck/Texture/king_of_diamonds.king_of_diamonds"))))))))