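; Card deck actor that builds a factory deck on BeginPlay, cuts it at a random index and Fisher-Yates shuffles it.
; RenderDeck spawns a BP_Display_BasicCard per card in a face-down vertical stack, while DisplayDeck spreads them over 13 columns.
; When IsRendering is set, both instead remove CardActorArray entries without destroying the actors.
; Neither is called here; the event graph also holds unwired calls to card and deck functions.
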(event EventBeginPlay
  (Class|StandardCardDeck|CreateFactoryDeck)
  (Class|StandardCardDeck|CutCards (Math|Random|RandomIntegerinRange 0 51))
  (Class|StandardCardDeck|FisherYatesShuffle))

(fn ConstructionScript)

(fn RenderDeck
  (bind _cardactorarray (Variables|Default|GetCardActorArray))
  (if (Variables|Default|GetbIsRendering)
    (for (_ _array_index) _cardactorarray
      (Utilities|Array|RemoveIndex _cardactorarray _array_index)
      (Variables|Default|SetbIsRendering true))
    (else
      (for (_array_element _array_index_2) (Utilities|Struct|BreakStandardCardArray (Variables|Default|GetDeck))
        (LocalVariables|SetLocal_Card _array_element)
        (LocalVariables|SetLocal_Index _array_index_2)
        (bind _returnvalue (Game|SpawnActorfromClass "/Game/DeckOfCards/Deck/BP_Display_BasicCard.BP_Display_BasicCard_C" (Math|Transform|MakeTransform (Math|Vector|MakeVector 0.0 0.0 (* (LocalVariables|GetLocal_Index) (Variables|CardDisplay|GetRenderCardSeperationBuffer)))) "Undefined" 0 (Math|Transform|MakeTransform (Math|Vector|MakeVector 0.0 0.0 (* (LocalVariables|GetLocal_Index) (Variables|CardDisplay|GetRenderCardSeperationBuffer)))) _array_element (Variables|CardDisplay|GetUseFaceCards) false))
        (Utilities|Array|Add (Variables|Default|GetCardActorArray) _returnvalue)
        (Variables|Default|SetbIsRendering true)))))

(fn DisplayDeck
  (bind _cardactorarray (Variables|Default|GetCardActorArray))
  (if (Variables|Default|GetbIsRendering)
    (for (_ _array_index) _cardactorarray
      (Utilities|Array|RemoveIndex _cardactorarray _array_index)
      (Variables|Default|SetbIsRendering false))
    (else
      (for (_array_element _array_index_2) (Utilities|Struct|BreakStandardCardArray (Variables|Default|GetDeck))
        (LocalVariables|SetLocal_Card _array_element)
        (LocalVariables|SetLocal_Index _array_index_2)
        (bind _returnvalue (Game|SpawnActorfromClass "/Game/DeckOfCards/Deck/BP_Display_BasicCard.BP_Display_BasicCard_C" (Math|Transform|MakeTransform (Math|Vector|MakeVector (* (Math|Float|%(Float) (Math|Conversions|ToFloat(Integer) (LocalVariables|GetLocal_Index)) 13.0) (Variables|CardDisplay|GetDisplayCardSeperationBuffer)) (* (/ (Math|Conversions|ToFloat(Integer) (LocalVariables|GetLocal_Index)) 13.0) (+ (Variables|CardDisplay|GetDisplayCardSeperationBuffer) 5e+01)) 0.0)) "AlwaysSpawn" 0 (Math|Transform|MakeTransform (Math|Vector|MakeVector (* (Math|Float|%(Float) (Math|Conversions|ToFloat(Integer) (LocalVariables|GetLocal_Index)) 13.0) (Variables|CardDisplay|GetDisplayCardSeperationBuffer)) (* (/ (Math|Conversions|ToFloat(Integer) (LocalVariables|GetLocal_Index)) 13.0) (+ (Variables|CardDisplay|GetDisplayCardSeperationBuffer) 5e+01)) 0.0)) (LocalVariables|GetLocal_Card) (Variables|CardDisplay|GetUseFaceCards) (Variables|CardDisplay|GetIsFaceUp)))
        (Utilities|Array|Add (Variables|Default|GetCardActorArray) _returnvalue)
        (Variables|Default|SetbIsRendering true)))))