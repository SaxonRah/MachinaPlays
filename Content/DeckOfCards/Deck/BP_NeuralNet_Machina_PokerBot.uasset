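; Neural-net poker bot that trains a small logistic network every tick to classify poker hand ranks.
; Each random hand becomes suit/rank inputs for forward propagation, and PokerGame's analyzed rank is the backpropagation target.
; Targets are raw rank integers, while the output is remapped to a rank for on-screen error and right/wrong tallies.
; An alternative trainer, GenerativeTrainingHelp, generates hands by random rank type but is never run.
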(event `self.ReceiveTick`
  (params (DeltaSeconds :type "Float (single-precision)"))
  (`self.GenerativeTrainingNoHelp`))

(event `self.ReceiveBeginPlay`
  (`self.Setup` (`|MakeArray` 10 5 1) "TT_Logistic" 0.15 0.5))

(fn `ConvertHandToTrainingHand`
  (params (`In Hand` :type "StandardCardArray Structure"))
  (`KismetArrayLibrary.Array_Clear` (`self.TrainingHand`))
  (bind _output_get (set `self.TempTrainingPokerHand` `In Hand`))
  (for _array_element (`.SCArray` (break `StandardCardArray` _output_get))
    (bind (_suit _rank) (break `StandardCard` _array_element))
    ;[1 1 1] Suit Rank
    (`KismetArrayLibrary.Array_Add` (`self.TrainingHand`) (`KismetMathLibrary.Conv_ByteToDouble` _suit))
    ;[1 1 1] Face Rank
    (`KismetArrayLibrary.Array_Add` (`self.TrainingHand`) (`KismetMathLibrary.Conv_ByteToDouble` _rank))))

(fn `DrawTrainingHand`
  (`KismetArrayLibrary.Array_Clear` (`self.TrainingHand`))
  (bind _outhand (`PokerGame.DrawPokerHandFromAnInfiniteDeck` (`self.PokerGame`)))
  (bind _output_get (set `self.TempTrainingPokerHand` _outhand))
  (for _array_element (`.SCArray` (break `StandardCardArray` _output_get))
    (bind (_suit _rank) (break `StandardCard` _array_element))
    ;[1 1 1] Suit Rank
    (`KismetArrayLibrary.Array_Add` (`self.TrainingHand`) (`KismetMathLibrary.Conv_ByteToDouble` _suit))
    ;[1 1 1] Face Rank
    (`KismetArrayLibrary.Array_Add` (`self.TrainingHand`) (`KismetMathLibrary.Conv_ByteToDouble` _rank))))

(fn `GenerativeTrainingHelp`
  (bind _idealhandoutput (`self.IdealHandOutput`))
  (bind _pokergame (`self.PokerGame`))
  (`|ExecutionSequence`
    (:`then_0`
      (bind _returnvalue (`PokerGame.RandomHandRank` _pokergame 0 8 :!label _label))
      (bind (_outhand _returnvalue_2) (`PokerGame.GeneratePokerHandByType` _pokergame _returnvalue))
      (set `self.TempTrainingPokerHand` _outhand)
      (if _returnvalue_2
        (`self.ConvertHandToTrainingHand` (`self.TempTrainingPokerHand`))
        (`self.ForwardPropagation` (`self.TrainingHand`))
        (bind _returnvalue_3 (`PokerGame.GetHandAsString` (`self.PokerGame`) (`self.TempTrainingPokerHand`)))
        (set `self.HandString` _returnvalue_3)
        (bind _returnvalue_4 (`PokerGame.AnalyzePokerHand` (`self.PokerGame`) (`self.TempTrainingPokerHand`)))
        (set `self.TempHandRank` _returnvalue_4)
        (`KismetArrayLibrary.Array_Clear` _idealhandoutput)
        (`KismetArrayLibrary.Array_Add` _idealhandoutput (`KismetMathLibrary.Conv_IntToDouble` (`KismetMathLibrary.Conv_ByteToInt` (`self.TempHandRank`))))
        (`self.BackwardPropagationOfErrors` (`self.IdealHandOutput`))
        (else
          (goto _label))))
    (:`then_1`
      (`KismetSystemLibrary.PrintString` (`KismetStringLibrary.Concat_StrStr` "Recent Average Error : " (`KismetStringLibrary.Conv_DoubleToString` (`self.GetRecentAverageError`))) true true (struct :`R` 1.0 :`A` 1.0) 0.0)
      (`KismetSystemLibrary.PrintString` (`KismetStringLibrary.Concat_StrStr` "Hand: " (`self.HandString`)) true true (struct :`R` 1.0 :`G` 1.0 :`A` 1.0) 0.0)
      (`KismetSystemLibrary.PrintString` (`KismetStringLibrary.Concat_StrStr` "Actual Hand Rank : " (`|GetEnumeratorNameAsString` (`self.TempHandRank`))) true true (struct :`G` 0.66 :`B` 1.0 :`A` 1.0) 0.0)
      (for (_array_element _array_index) (`self.GetResults`)
        (bind _output_get (set `self.TempNNHandRank` (cast `EStandardPokerHandRank` (`KismetMathLibrary.Conv_IntToByte` (`KismetMathLibrary.FTrunc` (`KismetMathLibrary.MapRangeClamped` _array_element 0.0 1.0 0.0 9.0))))))
        (`KismetSystemLibrary.PrintString` (`KismetStringLibrary.Concat_StrStr` "Result Of Network Output Neuron [ " (`KismetStringLibrary.Conv_IntToString` _array_index) " ] : " (`|GetEnumeratorNameAsString` _output_get)) true true (struct :`G` 1.0 :`A` 1.0) 0.0)))
    (:`then_2`
      (if (`|EnumEquality` (`self.TempNNHandRank`) (`self.TempHandRank`))
        (bind _output_get_2 (set `self.NumberCorrect` (+ (`self.NumberCorrect`) 1)))
        (`KismetSystemLibrary.PrintString` (`KismetStringLibrary.Concat_StrStr` "Number Correct : " (`KismetStringLibrary.Conv_IntToString` _output_get_2)) true true (struct :`G` 0.66 :`B` 1.0 :`A` 1.0) 0.0)
        (`KismetSystemLibrary.PrintString` (`KismetStringLibrary.Concat_StrStr` "Number Wrong : " (`KismetStringLibrary.Conv_IntToString` (`self.NumberWrong`))) true true (struct :`G` 0.66 :`B` 1.0 :`A` 1.0) 0.0)
        (else
          (`KismetSystemLibrary.PrintString` (`KismetStringLibrary.Concat_StrStr` "Number Correct : " (`KismetStringLibrary.Conv_IntToString` (`self.NumberCorrect`))) true true (struct :`G` 0.66 :`B` 1.0 :`A` 1.0) 0.0)
          (bind _output_get_3 (set `self.NumberWrong` (+ (`self.NumberWrong`) 1)))
          (`KismetSystemLibrary.PrintString` (`KismetStringLibrary.Concat_StrStr` "Number Wrong : " (`KismetStringLibrary.Conv_IntToString` _output_get_3)) true true (struct :`G` 0.66 :`B` 1.0 :`A` 1.0) 0.0))))))

(fn `GenerativeTrainingNoHelp`
  (bind _idealhandoutput (`self.IdealHandOutput`))
  (`|ExecutionSequence`
    (:`then_0`
      (`self.DrawTrainingHand`)
      (`self.ForwardPropagation` (`self.TrainingHand`))
      (bind _returnvalue (`PokerGame.GetHandAsString` (`self.PokerGame`) (`self.TempTrainingPokerHand`)))
      (set `self.HandString` _returnvalue)
      (bind _returnvalue_2 (`PokerGame.AnalyzePokerHand` (`self.PokerGame`) (`self.TempTrainingPokerHand`)))
      (set `self.TempHandRank` _returnvalue_2)
      (`KismetArrayLibrary.Array_Clear` _idealhandoutput)
      (`KismetArrayLibrary.Array_Add` _idealhandoutput (`KismetMathLibrary.Conv_IntToDouble` (`KismetMathLibrary.Conv_ByteToInt` (`self.TempHandRank`))))
      (`self.BackwardPropagationOfErrors` (`self.IdealHandOutput`)))
    (:`then_1`
      (`KismetSystemLibrary.PrintString` (`KismetStringLibrary.Concat_StrStr` "Recent Average Error : " (`KismetStringLibrary.Conv_DoubleToString` (`self.GetRecentAverageError`))) true true (struct :`R` 1.0 :`A` 1.0) 0.0)
      (`KismetSystemLibrary.PrintString` (`KismetStringLibrary.Concat_StrStr` "Hand: " (`self.HandString`)) true true (struct :`R` 1.0 :`G` 1.0 :`A` 1.0) 0.0)
      (`KismetSystemLibrary.PrintString` (`KismetStringLibrary.Concat_StrStr` "Actual Hand Rank : " (`|GetEnumeratorNameAsString` (`self.TempHandRank`))) true true (struct :`G` 0.66 :`B` 1.0 :`A` 1.0) 0.0)
      (for (_array_element _array_index) (`self.GetResults`)
        (bind _output_get (set `self.TempNNHandRank` (cast `EStandardPokerHandRank` (`KismetMathLibrary.Conv_IntToByte` (`KismetMathLibrary.FTrunc` (`KismetMathLibrary.MapRangeUnclamped` _array_element 0.0 1.0 0.0 9.0))))))
        (`KismetSystemLibrary.PrintString` (`KismetStringLibrary.Concat_StrStr` "Result Of Network Output Neuron [ " (`KismetStringLibrary.Conv_IntToString` _array_index) " ] : " (`|GetEnumeratorNameAsString` _output_get)) true true (struct :`G` 1.0 :`A` 1.0) 0.0)))
    (:`then_2`
      (if (`|EnumEquality` (`self.TempNNHandRank`) (`self.TempHandRank`))
        (bind _output_get_2 (set `self.NumberCorrect` (+ (`self.NumberCorrect`) 1)))
        (`KismetSystemLibrary.PrintString` (`KismetStringLibrary.Concat_StrStr` "Number Correct : " (`KismetStringLibrary.Conv_IntToString` _output_get_2)) true true (struct :`G` 0.66 :`B` 1.0 :`A` 1.0) 0.0)
        (`KismetSystemLibrary.PrintString` (`KismetStringLibrary.Concat_StrStr` "Number Wrong : " (`KismetStringLibrary.Conv_IntToString` (`self.NumberWrong`))) true true (struct :`G` 0.66 :`B` 1.0 :`A` 1.0) 0.0)
        (else
          (`KismetSystemLibrary.PrintString` (`KismetStringLibrary.Concat_StrStr` "Number Correct : " (`KismetStringLibrary.Conv_IntToString` (`self.NumberCorrect`))) true true (struct :`G` 0.66 :`B` 1.0 :`A` 1.0) 0.0)
          (bind _output_get_3 (set `self.NumberWrong` (+ (`self.NumberWrong`) 1)))
          (`KismetSystemLibrary.PrintString` (`KismetStringLibrary.Concat_StrStr` "Number Wrong : " (`KismetStringLibrary.Conv_IntToString` _output_get_3)) true true (struct :`G` 0.66 :`B` 1.0 :`A` 1.0) 0.0))))))

(fn `UserConstructionScript`)